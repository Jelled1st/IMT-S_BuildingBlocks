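; 3D actor that displays Formula 1 team data in a widget list once sports API data loads.
; On BeginPlay it gets the sport data handler from the CoreSystem game instance and binds to its event system's data-loaded delegate.
; The callback converts each team's score, nationality and player count into a UI struct with fixed textures, stores it, and forwards it to WBP_F1_ListView.
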(event `self.ReceiveBeginPlay`
  (bind _ascore_system (cast `CoreSystem` (`GameplayStatics.GetGameInstance`)))
  (bind _output_get (set `self.CoreSystemInstance` _ascore_system))
  (add `EventSystem.apiDataLoadedDelegate` (`CoreSystem.GetEventSystem` _output_get) (delegate `Event_ApiDataLoaded`))
  (bind _returnvalue (`CoreSystem.GetBPSportDataHandler` _output_get))
  (set `self.DataHandler` _returnvalue))

(event `Event_ApiDataLoaded`
  (params (sport :type "Sport Enum" :default "Cricket"))
  (`KismetSystemLibrary.PrintString` "Callback received from BP")
  (bind _returnvalue (`SportDataHandler.GetF1Teams` (`self.DataHandler`)))
  (for _array_element _returnvalue
    (bind _returnvalue_2 (`Team.GetScore` _array_element))
    (bind _returnvalue_3 (`Team.GetNationalityAsString` _array_element))
    (bind _returnvalue_4 (`Team.GetPlayers` _array_element))
    (`self.AddF1StructToList` (make `/Game/Blueprints/F1TeamData/UMG_Teams` _returnvalue_2 (`KismetTextLibrary.Conv_StringToText` _returnvalue_3) (`KismetArrayLibrary.Array_Length` _returnvalue_4) "/Game/Assets/UI/Modular_UI_assets/Asset_25.Asset_25" "/Game/Assets/UI/Modular_UI_assets/Team_name_red.Team_name_red" "/Game/Assets/UI/Modular_UI_assets/Nr_red.Nr_red"))))

(fn `AddF1StructToList`
  (params (`New Data` :type "/Game/Blueprints/F1TeamData/UMG_Teams Structure"))
  (`KismetArrayLibrary.Array_Add` (`self.F1 Data Array`) `New Data`)
  (bind _aswbp_f1_list_view (cast `/Game/Blueprints/F1TeamData/WBP_F1_ListView` (`WidgetComponent.GetWidget` (`self.Widget`))))
  (`/Game/Blueprints/F1TeamData/WBP_F1_ListView.AddF1Data To List` _aswbp_f1_list_view `New Data`))

(fn `UserConstructionScript`)