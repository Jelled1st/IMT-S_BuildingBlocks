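; Component that shifts the hue of its owner's static mesh material according to an elevator actor's height between floor actors.
; BeginPlay creates a dynamic material instance, or prints an error and quits the game if the floor and hue arrays differ in length.
; Each tick finds the adjacent floor pair bracketing the elevator's Z, linearly interpolates their hue values and sets the HueShift parameter.
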(event `self.ReceiveBeginPlay`
  (bind _hueshiftmaterialindex (`self.hueShiftMaterialIndex`))
  (bind _returnvalue (`Actor.GetComponentByClass` (`self.GetOwner`) "/Script/Engine.StaticMeshComponent"))
  (if (== (`KismetArrayLibrary.Array_Length` (`self.elevatorFloors`)) (`KismetArrayLibrary.Array_Length` (`self.floorHueShifts`)))
    (bind _returnvalue_2 (`PrimitiveComponent.CreateDynamicMaterialInstance` _returnvalue _hueshiftmaterialindex (`PrimitiveComponent.GetMaterial` _returnvalue _hueshiftmaterialindex) "None"))
    (set `self.hueShiftMaterialDynamic` _returnvalue_2)
    (else
      (`KismetSystemLibrary.PrintText` "ElevatorFloors and floorHueShifts not equal")
      (`KismetSystemLibrary.QuitGame` null "Quit"))))

(event `self.ReceiveTick`
  (params (DeltaSeconds :type "Float (single-precision)"))
  (bind _elevatorfloors (`self.elevatorFloors`))
  (for (_array_element _array_index) _elevatorfloors
    (`/Engine/EditorBlueprintResources/StandardMacros.CompareInt` _array_index (- (`KismetArrayLibrary.Array_Length` _elevatorfloors) 1)
      (:`==`
        (break))
      (:`<`
        (bind _posz (`self.GetActorPosZ` (`self.elevatorActor`)))
        (bind _output (`|GetArrayItem` _elevatorfloors (+ _array_index 1)))
        (bind _isbetweenfloors (`self.IsElevatorBetweenFloors` _posz _array_element _output))
        (if _isbetweenfloors
          (bind _posz_2 (`self.GetActorPosZ` _array_element))
          (bind _posz_3 (`self.GetActorPosZ` _output))
          (bind _procentage (`self.GetProcentageBetweenFloors` _posz _posz_2 _posz_3))
          (bind _hueshift (`self.GetHueShift` _procentage _array_index (+ _array_index 1)))
          (`MaterialInstanceDynamic.SetScalarParameterValue` (`self.hueShiftMaterialDynamic`) "HueShift" _hueshift))))))

(fn `GetActorPosZ`
  (params (actor :type "Actor Object Reference"))
  (returns (posZ :type "Float (double-precision)"))
  (return (.z (`Actor.K2_GetActorLocation` actor))))

(fn `GetHueShift`
  (params (mixProcent :type "Float (double-precision)") (floor0Index :type Integer) (floor1Index :type Integer))
  (returns (hueShift :type "Float (double-precision)"))
  (bind _floorhueshifts (`self.floorHueShifts`))
  (bind _output (`|GetArrayItem` _floorhueshifts floor0Index))
  (return (+ _output (* (- (`|GetArrayItem` _floorhueshifts floor1Index) _output) mixProcent))))

(fn `GetProcentageBetweenFloors`
  (params (elevatorZ :type "Float (double-precision)") (floor0Z :type "Float (double-precision)") (floor1Z :type "Float (double-precision)"))
  (returns (procentage :type "Float (double-precision)"))
  (return (/ (- elevatorZ floor0Z) (- floor1Z floor0Z))))

(fn `IsElevatorBetweenFloors`
  (params (elevatorPositionZ :type "Float (double-precision)") (floor0 :type "Actor Object Reference") (floor1 :type "Actor Object Reference"))
  (returns (isBetweenFloors :type Boolean))
  (bind _posz (`self.GetActorPosZ` floor0))
  (bind _posz_2 (`self.GetActorPosZ` floor1))
  (`/Engine/EditorBlueprintResources/StandardMacros.CompareFloat` _posz elevatorPositionZ
    (:`>`
      _)
    (:`==`
      _)
    (:`<`
      (`/Engine/EditorBlueprintResources/StandardMacros.CompareFloat` _posz_2 elevatorPositionZ
        (:`>`
          _)
        (:`==`
          _)
        (:`<`
          (return false)))
      (return true)))
  (return false))