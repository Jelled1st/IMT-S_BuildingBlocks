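; GridSpawner is a test actor that builds a flat grid of actors at BeginPlay from Width and Height.
; Nested loops place cells at fixed spacing in world coordinates, alternating GridElementTest and GridElementTest2 by the parity of the Y index.
; Each GridElementTest also gets a separately spawned, movable StaticMeshActor at its location, with a cylinder mesh assigned at runtime.
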(event `self.ReceiveBeginPlay`
  (for _index (range (+ (`self.Width`) 1))
    (for _index_2 (range (+ (`self.Height`) 1))
      (bind _returnvalue (`KismetMathLibrary.MakeTransform` (`KismetMathLibrary.MakeVector` (`KismetMathLibrary.Conv_IntToDouble` (* _index 300)) (`KismetMathLibrary.Conv_IntToDouble` (* _index_2 300)))))
      (set `self.NewVar_0` _returnvalue)
      (if (== (mod _index_2 2) 0)
        (bind _returnvalue_2 (`|SpawnActorFromClass` "/Game/Blueprints/GridTest/GridElementTest.GridElementTest_C" _returnvalue "Undefined" "OverrideRootScale" null null))
        (bind _returnvalue_3 (`|SpawnActorFromClass` "/Script/Engine.StaticMeshActor" (`KismetMathLibrary.Conv_VectorToTransform` (`self.K2_GetActorLocation` _returnvalue_2)) "Undefined" "OverrideRootScale" null null))
        (`StaticMeshActor.SetMobility` _returnvalue_3 "Movable")
        (`StaticMeshComponent.SetStaticMesh` (`StaticMeshActor.StaticMeshComponent` _returnvalue_3) "/Game/Assets/UI/Aylas_UI_assets/3D_UI_Cylinder001.3D_UI_Cylinder001")
        (else
          (`|SpawnActorFromClass` "/Game/Blueprints/GridTest/GridElementTest2.GridElementTest2_C" _returnvalue "Undefined" "OverrideRootScale" null null))))))

(fn `UserConstructionScript`)